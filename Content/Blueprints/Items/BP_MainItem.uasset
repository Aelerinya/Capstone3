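; BP_MainItem is an interactable world item that serves as a pickup, door or enigma.
; Overlapping its sphere shows an interact prompt, after a one-time tutorial if pending, and sets the matching ability flag and object reference on BP_MyPlayer.
; Leaving the sphere removes the prompt and clears them.
; Doors open through a looping timer that lerps the mesh toward a 90-degree yaw offset cached at BeginPlay.
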(event `self.ReceiveBeginPlay`
  (bind (_returnvalue_roll _returnvalue_pitch _returnvalue_yaw) (`KismetMathLibrary.BreakRotator` (`SceneComponent.K2_GetComponentRotation` (`self.StaticMesh`))))
  (set `self.OpenDoorRot` (`KismetMathLibrary.MakeRotator` _returnvalue_roll _returnvalue_pitch (+ _returnvalue_yaw 90.0))))

(event `self.Sphere.OnComponentBeginOverlap`
  (params (OverlappedComponent :type "PrimitiveComponent Object Reference") (OtherActor :type "Actor Object Reference") (OtherComp :type "PrimitiveComponent Object Reference") (OtherBodyIndex :type Integer) (bFromSweep :type Boolean) (SweepResult :type "HitResult Structure (by ref)"))
  (bind _tutoref (`self.TutoRef`))
  (if (`self.CanBeInteracted?`)
    (bind _asbp_my_player (cast `/Game/Blueprints/Player/BP_MyPlayer` OtherActor))
    (bind _output_get (set `self.PlayerRef` _asbp_my_player))
    (if (`/Game/Blueprints/Player/BP_MyPlayer.DisplayTutoUseItem?` _output_get)
      (set `/Game/Blueprints/Player/BP_MyPlayer.DisplayTutoUseItem?` false _output_get)
      (bind _returnvalue (`|CreateWidget` "/Game/Blueprints/Widget/WBP_Tuto.WBP_Tuto_C"))
      (bind _output_get_2 (set `self.TutoRef` _returnvalue))
      (`UserWidget.AddToViewport` _output_get_2 0)
      (`/Game/Blueprints/Widget/WBP_Tuto.SetTutoText` _tutoref "Press E to interact with items doors keys etc")
      (add `/Game/Blueprints/Widget/WBP_Tuto.TutoRemoving` _tutoref (delegate `DisplayInteract`))
      (else
        (bind _returnvalue_2 (`|CreateWidget` "/Game/Blueprints/Widget/WBP_Interact.WBP_Interact_C" :!label _label))
        (bind _output_get_3 (set `self.InteractRef` _returnvalue_2))
        (`UserWidget.AddToViewport` _output_get_3 0)
        (`/Game/Blueprints/Widget/WBP_Interact.SetInteractText` _output_get_3 (`self.Name`))
        (set `/Game/Blueprints/Player/BP_MyPlayer.InteractObject` self (`self.PlayerRef`))
        (if (`self.PickUpItems?`)
          (set `/Game/Blueprints/Player/BP_MyPlayer.CanPickUp?` true (`self.PlayerRef`))
          (set `/Game/Blueprints/Player/BP_MyPlayer.InteractRef` (`self.InteractRef`) (`self.PlayerRef`) :!label _label_2)
          (elif (`self.Door?`)
            (set `/Game/Blueprints/Player/BP_MyPlayer.CanUseDoor?` true (`self.PlayerRef`))
            (goto _label_2)
            (elif (`self.Enigma`)
              (set `/Game/Blueprints/Player/BP_MyPlayer.CanUseEnigma?` true (`self.PlayerRef`))
              (goto _label_2))))))))

(event `DisplayInteract`
  (goto _label))

(event `RemoveInteractWidget`
  (bind _interactref (`self.InteractRef`))
  (bind _playerref (`self.PlayerRef`))
  (`/Engine/EditorBlueprintResources/StandardMacros.IsValid` _interactref :!label _label_3
    (:`Is Valid`
      (`Widget.RemoveFromParent` _interactref))
    (:`Is Not Valid`
      _))
  (`/Engine/EditorBlueprintResources/StandardMacros.IsValid` _playerref
    (:`Is Valid`
      (set `/Game/Blueprints/Player/BP_MyPlayer.CanPickUp?` false _playerref)
      (set `/Game/Blueprints/Player/BP_MyPlayer.InteractObject` null _playerref)
      (set `/Game/Blueprints/Player/BP_MyPlayer.CanUseDoor?` false _playerref)
      (set `/Game/Blueprints/Player/BP_MyPlayer.CanUseEnigma?` false _playerref))))

(event `self.Sphere.OnComponentEndOverlap`
  (params (OverlappedComponent :type "PrimitiveComponent Object Reference") (OtherActor :type "Actor Object Reference") (OtherComp :type "PrimitiveComponent Object Reference") (OtherBodyIndex :type Integer))
  (goto _label_3))

(event `StartOpeningDoor`
  (`KismetSystemLibrary.K2_SetTimer` null "OpenDoor" 0.01 true)
  (`self.BigDoorOpened`))

(fn `OpenDoor`
  (bind _opendoorrot (`self.OpenDoorRot`))
  (bind _returnvalue (`KismetMathLibrary.RLerp` (`SceneComponent.K2_GetComponentRotation` (`self.StaticMesh`)) _opendoorrot 0.01))
  (`SceneComponent.K2_SetWorldRotation` (`self.StaticMesh`) _returnvalue false false)
  (if (== _returnvalue _opendoorrot :`ErrorTolerance` 5.0)
    (`KismetSystemLibrary.K2_ClearTimer` null "OpenDoor")))

(fn `UserConstructionScript`)