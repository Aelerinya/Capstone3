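; BP_StaticCamera is a fixed camera actor that the player's view can switch to and away from.
; EnterCamera registers it as BP_MyPlayer's CurrentStaticCamera, makes it the view target and aligns control rotation to the camera's yaw.
; LeaveCamera returns the view to the player and clears that reference, but only if this camera is still current, so a newer camera is not overridden.
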(event `EnterCamera`
  (bind _returnvalue (`GameplayStatics.GetPlayerController` 0))
  (bind (_returnvalue_roll _returnvalue_pitch _returnvalue_yaw) (`KismetMathLibrary.BreakRotator` (`SceneComponent.K2_GetComponentRotation` (`self.CameraComponent`))))
  (bind _asbp_my_player (cast `/Game/Blueprints/Player/BP_MyPlayer` (`GameplayStatics.GetPlayerPawn` 0)))
  (set `/Game/Blueprints/Player/BP_MyPlayer.CurrentStaticCamera` self _asbp_my_player)
  (`PlayerController.SetViewTargetWithBlend` _returnvalue self 0.0 "VTBlend_Linear" 0.0 false)
  (`Controller.SetControlRotation` _returnvalue (`KismetMathLibrary.MakeRotator` 0.0 0.0 _returnvalue_yaw)))

(event `LeaveCamera`
  (bind _asbp_my_player (cast `/Game/Blueprints/Player/BP_MyPlayer` (`GameplayStatics.GetPlayerPawn` 0)))
  (if (== (`/Game/Blueprints/Player/BP_MyPlayer.CurrentStaticCamera` _asbp_my_player) self)
    (`PlayerController.SetViewTargetWithBlend` (`GameplayStatics.GetPlayerController` 0) _asbp_my_player 0.0 "VTBlend_Linear" 0.0 false)
    (set `/Game/Blueprints/Player/BP_MyPlayer.CurrentStaticCamera` null _asbp_my_player)))

(fn `UserConstructionScript`)